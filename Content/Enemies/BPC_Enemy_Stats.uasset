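; BPC_Enemy_Stats is an enemy stats component that tracks health and drives the owning BP_Enemy's health bar.
; DecreasHealth subtracts damage, updates the bar to current over maximum health, and returns true once health is at or below zero.
; The owner cast and initial bar update sit in disconnected nodes, so nothing in these graphs that runs assigns the AsBPEnemy reference DecreasHealth uses.
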(event `self.ReceiveBeginPlay`)

(fn `DecreasHealth`
  (params (Damage :type "Float (double-precision)"))
  (returns (IsEnemyDead :type Boolean))
  (if (not (<= (`self.CurrentHealth`) 0.0))
    (bind _output_get (set `self.CurrentHealth` (- (`self.CurrentHealth`) Damage)))
    (`ProgressBar.SetPercent` (`/Game/UI/WB_EnemyHealthbar.Healthbar` (`/Game/Enemies/BP_Enemy.Healt widget` (`self.As BP Enemy`))) (/ _output_get (`self.MaxHealth`)))
    (if (<= (`self.CurrentHealth`) 0.0)
      _
      (else
        (return false))))
  (return true))