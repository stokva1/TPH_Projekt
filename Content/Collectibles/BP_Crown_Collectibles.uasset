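; BP_Crown_Collectibles is a crown pickup that counts toward the player's collected items.
; It starts hidden with actor collision off, and nothing in this Blueprint re-enables it.
; When an actor tagged Player overlaps its Sphere, it casts to ThirdPersonCharacter and updates the mission text to send the player to another location.
; It then destroys itself and increments the character's ItemsCollected.
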(event `self.ReceiveBeginPlay`
  (`self.SetActorEnableCollision` false)
  (`self.SetActorHiddenInGame` true))

(event `self.Sphere.OnComponentBeginOverlap`
  (params (OverlappedComponent :type "PrimitiveComponent Object Reference") (OtherActor :type "Actor Object Reference") (OtherComp :type "PrimitiveComponent Object Reference") (OtherBodyIndex :type Integer) (bFromSweep :type Boolean) (SweepResult :type "HitResult Structure (by ref)"))
  (if (`self.ActorHasTag` OtherActor "Player")
    (bind _asthird_person_character (cast `/Game/ThirdPersonBP/Blueprints/ThirdPersonCharacter` OtherActor))
    (`/Game/ThirdPersonBP/Blueprints/ThirdPersonCharacter.UpdateMission` _asthird_person_character "Great you found the item! Now go find another location to clear")
    (`self.K2_DestroyActor`)
    (bind _result (`/Engine/EditorBlueprintResources/StandardMacros.IncrementInt` (`/Game/ThirdPersonBP/Blueprints/ThirdPersonCharacter.ItemsCollected` _asthird_person_character))
      (:`  `
        (set `/Game/ThirdPersonBP/Blueprints/ThirdPersonCharacter.ItemsCollected` _result _asthird_person_character)))))

(fn `UserConstructionScript`)