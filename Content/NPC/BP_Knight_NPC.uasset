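; Knight NPC that plays a looping unarmed idle and holds a dialogue with the player, ending in a mission update.
; Each Talk call advances through the Dialogue array, showing the line in a lazily created WB_Dialogue widget and disabling player movement.
; Past the last line it removes the widget, restores walking and, through a DoOnce, passes its Mission to ThirdPersonCharacter's UpdateMission.
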(event `self.ReceiveBeginPlay`
  (`SkeletalMeshComponent.PlayAnimation` (`self.Mesh`) "/Game/NPC/Unarmed_Idle_01.Unarmed_Idle_01" true))

(event `/Game/NPC/BPI_Dialog.Talk`
  (bind _returnvalue (`GameplayStatics.GetPlayerCharacter` 0))
  (`/Engine/EditorBlueprintResources/StandardMacros.IncrementInt` (`self.TalkIndex`)
    (:`  `
      (if (< (`self.TalkIndex`) (`KismetArrayLibrary.Array_Length` (`self.Dialogue`)))
        (`self.UI`
          (:`then`
            _)
          (:`else`
            (bind _returnvalue_2 (`|CreateWidget` "/Game/UI/WB_Dialogue.WB_Dialogue_C" (`GameplayStatics.GetPlayerController` 0)))
            (bind _output_get (set `self.UI` _returnvalue_2))
            (`UserWidget.AddToViewport` _output_get 0)))
        (`TextBlock.SetText` (`/Game/UI/WB_Dialogue.TalkText` (`self.UI`)) (`KismetTextLibrary.Conv_StringToText` (`|GetArrayItem` (`self.Dialogue`) (`self.TalkIndex`))))
        (`CharacterMovementComponent.DisableMovement` (`Character.CharacterMovement` (`GameplayStatics.GetPlayerCharacter` 0)))
        (else
          (`Widget.RemoveFromParent` (`self.UI`))
          (`CharacterMovementComponent.SetMovementMode` (`Character.CharacterMovement` _returnvalue) "MOVE_Walking" 0)
          (bind _asthird_person_character (cast `/Game/ThirdPersonBP/Blueprints/ThirdPersonCharacter` _returnvalue))
          (`/Engine/EditorBlueprintResources/StandardMacros.DoOnce` false
            (:`Completed`
              (`/Game/ThirdPersonBP/Blueprints/ThirdPersonCharacter.UpdateMission` _asthird_person_character (`self.Mission`)))))))))

(fn `UserConstructionScript`)